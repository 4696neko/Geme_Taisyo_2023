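; BP_TestInstance is a prototype data holder that fills in hard-coded test data for an RPG-style battle.
; CreateCharacter builds stat structs for Hero, EnemyA and EnemyB, flags the enemies, and collects all three into SpdStruct without sorting.
; Two setup functions fill Player 1's special-attack list with MP costs and item list with attack values, using Japanese names.
; It contains only data setup, with no combat logic.
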(fn `Create_Character`
  (set `self.Hero` (make `/Game/ProtoTest/BP/BP_Player` "Hero" 100 100 10 10 10 10 10 10 10 10))
  (set `self.EnemyA` (make `/Game/ProtoTest/BP/BP_Player` "EnemyA" 100 100 10 10 10 10 10 10 10 10 1.0 true))
  (set `self.EnemyB` (make `/Game/ProtoTest/BP/BP_Player` "EnemyB" 50 50 10 10 10 10 20 20 10 10 1.0 true))
  (set `self.Spd_Struct` (`|MakeArray` (`self.Hero`) (`self.EnemyA`) (`self.EnemyB`))))

(fn `Set_Player1_Item`
  (set `self.Player1_Item` (`|MakeArray` (make `/Game/ProtoTest/BP/BP_Item` "モロトフ" 30 0 0 1.0 20) (make `/Game/ProtoTest/BP/BP_Item` "回復薬" 0 70 0 1.0 999) (make `/Game/ProtoTest/BP/BP_Item` "魔力回復薬" 0 70 30 1.0 999) (make `/Game/ProtoTest/BP/BP_Item` "怪力の丸薬" 0 0 0 2.0 999 1.0 true) (make `/Game/ProtoTest/BP/BP_Item` "鎮痛剤" 0 10 0 1.0 999 1.5 true) (struct))))

(fn `SetPlayer1_Special`
  (set `self.Player1_Sp` (`|MakeArray` (make `/Game/ProtoTest/BP/BP_SpecialAtk` "ふれいむ" 10 20 1.0 20) (make `/Game/ProtoTest/BP/BP_SpecialAtk` "ためる" 5 0 2.0 30 1.0 0 1.0 0 1.0 true false 1) (make `/Game/ProtoTest/BP/BP_SpecialAtk` "きりつける" 5 50 1.0 10) (make `/Game/ProtoTest/BP/BP_SpecialAtk` "いやす" 10 0 1.0 10 1.0 0 1.0 40 1.0 true) (make `/Game/ProtoTest/BP/BP_SpecialAtk` "きゅうしょづき" 15 50 1.0 20))))