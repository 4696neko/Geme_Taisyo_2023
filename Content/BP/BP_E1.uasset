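; BP_E1 is an enemy Blueprint that registers its combat stats with the shared BP_GameInstance.
; Set_Character_Speed writes its Agility as the character speed, then calls SetSpeed on the instance.
; Set_Date packs an "Enemy" tag, name and stats into CharactorDate, then calls AddDate.
; BeginPlay, overlap, Tick and the construction script are empty, and nothing in this graph calls the two custom events.
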(event `self.ReceiveBeginPlay`)

(event `Set_Character_Speed`
  (bind _asbp_game_instance (cast `/Game/BP/BP_GameInstance` (`GameplayStatics.GetGameInstance`) :!pure true))
  (set `/Game/BP/BP_GameInstance.Character_Speed` (`self.Agility`) _asbp_game_instance)
  (`/Game/BP/BP_GameInstance.Set Speed` _asbp_game_instance))

(event `Set_Date`
  (bind _asbp_game_instance (cast `/Game/BP/BP_GameInstance` (`GameplayStatics.GetGameInstance`) :!pure true))
  (set `/Game/BP/BP_GameInstance.Charactor_Date` (make `/Game/BP/BP_Charactor_Struct` "Enemy" (`self.Name`) (`self.HP`) (`self.MP`) (`self.Attack`) (`self.Defense`) (`self.Agility`)) _asbp_game_instance)
  (`/Game/BP/BP_GameInstance.Add_Date` _asbp_game_instance))

(fn `UserConstructionScript`)