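; BP_P3 is the third player character, a provisional thief, in a turn-based battle, with hardcoded stats set on BeginPlay.
; Tick shows HP/MP text by GameInstance turn and command, and destroys the actor at zero HP.
; Events scale attack, special and defense by rates and apply defense-reduced damage to paired HP/MP bar widgets.
; Set_Date registers stats with BP_GameInstance, while Reset_Date applies damage from its character array and writes stats back.
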(event `self.ReceiveBeginPlay`
  ;[1 1 1] 盗賊(仮)
  (set `self.Name` "To-zoku_23")
  (set `self.HP` 30)
  (set `self.MP` 8)
  (set `self.Attack` 15)
  (set `self.Defense` 10)
  (set `self.Agility` 23)
  (bind _ashpbar_ui (cast `/Game/UI/HPBar_UI` (`WidgetComponent.GetUserWidgetObject` (`self.HPBar`))))
  (set `self.P3_HPBar_Ref` _ashpbar_ui)
  (bind _ashpbar_ui_2 (cast `/Game/UI/HPBar_UI` (`WidgetComponent.GetUserWidgetObject` (`self.HPBar2`))))
  (set `self.P3_HPBar2` _ashpbar_ui_2)
  (bind _asmpbar_ui (cast `/Game/UI/MPBar_UI` (`WidgetComponent.GetUserWidgetObject` (`self.MPBar`))))
  (set `self.P3_MPBar_Ref` _asmpbar_ui)
  (bind _asmpbar_ui_2 (cast `/Game/UI/MPBar_UI` (`WidgetComponent.GetUserWidgetObject` (`self.MPBar2`))))
  (set `self.P3_MPBar_Ref2` _asmpbar_ui_2))

(event `self.ReceiveTick`
  (params (DeltaSeconds :type "Float (single-precision)"))
  (bind _hp (`self.HP`))
  (if (<= _hp 0)
    (set `self.P3_Dead_Flg` true)
    (`self.K2_DestroyActor`)
    (else
      (`TextRenderComponent.K2_SetText` (`self.HP_text`) (`KismetTextLibrary.Conv_StringToText` (`KismetStringLibrary.Concat_StrStr` "HP" (`KismetTextLibrary.Conv_TextToString` (`KismetTextLibrary.Conv_IntToText` _hp)) "/" (`KismetTextLibrary.Conv_TextToString` (`KismetTextLibrary.Conv_IntToText` (`self.default_HP`))))))
      (`TextRenderComponent.K2_SetText` (`self.MP_text`) (`KismetTextLibrary.Conv_StringToText` (`KismetStringLibrary.Concat_StrStr` "MP" (`KismetTextLibrary.Conv_TextToString` (`KismetTextLibrary.Conv_IntToText` (`self.MP`))) "/" (`KismetTextLibrary.Conv_TextToString` (`KismetTextLibrary.Conv_IntToText` (`self.default_MP`))))))
      (if (== (`/Game/BP/BP_GameInstance.Player_Turn` (cast `/Game/BP/BP_GameInstance` (`GameplayStatics.GetGameInstance`) :!pure true)) 2)
        (if (`KismetMathLibrary.InRange_FloatFloat` (`KismetMathLibrary.Conv_IntToDouble` (`/Game/BP/BP_GameInstance.Command` (cast `/Game/BP/BP_GameInstance` (`GameplayStatics.GetGameInstance`) :!pure true))))
          (`SceneComponent.SetVisibility` (`self.Status_Back`) true false)
          (`SceneComponent.SetVisibility` (`self.HP_text`) true false)
          (`SceneComponent.SetVisibility` (`self.MP_text`) true false)
          (else
            (`SceneComponent.SetVisibility` (`self.Status_Back`) false false :!label _label)
            (`SceneComponent.SetVisibility` (`self.HP_text`) false false)
            (`SceneComponent.SetVisibility` (`self.MP_text`) false false)))
        (else
          (goto _label))))))

(event `Set_Date`
  (bind _asbp_game_instance (cast `/Game/BP/BP_GameInstance` (`GameplayStatics.GetGameInstance`) :!pure true))
  (set `/Game/BP/BP_GameInstance.Charactor_Date` (make `/Game/BP/BP_Charactor_Struct` "Player" (`self.Name`) (`self.Number`) (`self.default_HP`) (`self.default_MP`) (`self.default_Attack`) (`self.default_Defense`) (`self.default_Agility`)) _asbp_game_instance)
  (`/Game/BP/BP_GameInstance.Add_Date` _asbp_game_instance))

(event `Atk_Damege_Count`
  (set `self.Damege_Num` (`KismetMathLibrary.FTrunc` (* (`self.Attack`) (`self.Atk_Rate`)))))

(event `Spc_Damege_Count`
  (set `self.Damege_Num` (`KismetMathLibrary.FTrunc` (* (`self.Attack`) (`self.Spc_Rate`)))))

(event `Damege_calculation`
  (params (DamegeCount :type Integer))
  (bind _returnvalue (- DamegeCount (`self.Defense`)))
  (bind _returnvalue_2 (/ (`self.HP`) (`self.default_HP`)))
  (bind _returnvalue_3 (/ (`self.MP`) (`self.default_MP`)))
  (if (> _returnvalue 0)
    (set `self.HP` (- (`self.HP`) _returnvalue))
    (`/Game/UI/HPBar_UI.UpdateHealthProgress` (`self.P3_HPBar_Ref`) (`KismetMathLibrary.Conv_IntToDouble` _returnvalue_2) :!label _label_2)
    (`/Game/UI/HPBar_UI.UpdateHealthProgress` (`self.P3_HPBar2`) (`KismetMathLibrary.Conv_IntToDouble` _returnvalue_2))
    (`/Game/UI/MPBar_UI.UpdateMagicProgress` (`self.P3_MPBar_Ref`) (`KismetMathLibrary.Conv_IntToDouble` _returnvalue_3))
    (`/Game/UI/MPBar_UI.UpdateMagicProgress` (`self.P3_MPBar_Ref2`) (`KismetMathLibrary.Conv_IntToDouble` _returnvalue_3))
    (elif (< _returnvalue 0)
      (set `self.HP` (- (`self.HP`) 1))
      (goto _label_2))))

(event `Defence_Count`
  (set `self.Defense` (`KismetMathLibrary.FTrunc` (* (`self.Defense`) (`self.Def_Rate`)))))

(event `Reset_Date`
  (bind _charactor_array (`/Game/BP/BP_GameInstance.Charactor_Array` (cast `/Game/BP/BP_GameInstance` (`GameplayStatics.GetGameInstance`) :!pure true)))
  (for _array_element _charactor_array
    (`self.Damege_calculation` (`.Damege_count_40_9558AFDE40EA99874F23CC82DEB6C59F` (break `/Game/BP/BP_Charactor_Struct` _array_element)))
    (`KismetArrayLibrary.Array_Set` _charactor_array (`KismetArrayLibrary.Array_Find` _charactor_array (make `/Game/BP/BP_Charactor_Struct` "Player" (`self.Name`) (`self.Number`) (`.HP_10_9B2ED28144BB3F6249BEF582ED88F4DF` (break `/Game/BP/BP_Charactor_Struct` _array_element)) (`.MP_11_E06FDD2E4AE1539C2EC469B09C87921B` (break `/Game/BP/BP_Charactor_Struct` _array_element)) (`.Attack_21_DCBAB4424D4759E7446D4E9A1E0DEB9B` (break `/Game/BP/BP_Charactor_Struct` _array_element)) (`.Defense_22_706C65054E87FDCC3C347B9975D5EC03` (break `/Game/BP/BP_Charactor_Struct` _array_element)) (`.Agility_14_F6A6140546DC6CEBB2A6A79CEF8180B3` (break `/Game/BP/BP_Charactor_Struct` _array_element)) (`.command_num_31_36B8FD014313D156257521887835333F` (break `/Game/BP/BP_Charactor_Struct` _array_element)) (`.Tagetnum_37_E4975B044A8384EAE7EE34A8046078DC` (break `/Game/BP/BP_Charactor_Struct` _array_element)) (`.Damege_count_40_9558AFDE40EA99874F23CC82DEB6C59F` (break `/Game/BP/BP_Charactor_Struct` _array_element)))) (make `/Game/BP/BP_Charactor_Struct` "Player" (`self.Name`) (`self.Number`) (`self.HP`) (`self.MP`) (`self.default_Attack`) (`self.default_Defense`) (`self.default_Agility`)))))

(fn `UserConstructionScript`)