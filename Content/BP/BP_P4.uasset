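; BP_P4 is a player character definition for a placeholder Thief, holding its name and RPG stats.
; BeginPlay fills in hard-coded HP, MP, attack, defense and agility values.
; The Set_Date event packs them with a "Player" label and a false flag into BP_GameInstance's CharactorDate, then calls AddDate on that instance to register the character.
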(event `self.ReceiveBeginPlay`
  ;[1 1 1] 盗賊(仮)
  (set `self.Name` "To-zoku_23")
  (set `self.HP` 30)
  (set `self.MP` 8)
  (set `self.Attack` 15)
  (set `self.Defense` 10)
  (set `self.Agility` 23))

(event `Set_Date`
  (bind _asbp_game_instance (cast `/Game/BP/BP_GameInstance` (`GameplayStatics.GetGameInstance`) :!pure true))
  (set `/Game/BP/BP_GameInstance.Charactor_Date` (make `/Game/BP/BP_Charactor_Struct` "Player" (`self.Name`) (`self.HP`) (`self.MP`) (`self.Attack`) (`self.Defense`) (`self.Agility`)) _asbp_game_instance)
  (`/Game/BP/BP_GameInstance.Add_Date` _asbp_game_instance))

(fn `UserConstructionScript`)