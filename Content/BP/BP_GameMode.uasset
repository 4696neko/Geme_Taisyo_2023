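; Battle game mode that sets speed-based turn order from speed arrays held in BP_GameInstance.
; On BeginPlay it resets PlayerNum, builds SpeedArray0 by repeatedly taking the maximum of SpeedArray and clearing that slot, then prints the first four entries.
; Normal-attack and special-skill events scale the current player's sorted speed, leaving it unchanged or halving it respectively, then advance PlayerNum.
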(event `self.ReceiveBeginPlay`
  (`self.Roll_spd`))

(event `Sort_Speed`
  (bind _speed_array (`/Game/BP/BP_GameInstance.Speed_Array` (cast `/Game/BP/BP_GameInstance` (`GameplayStatics.GetGameInstance`) :!pure true)))
  (bind (_indexofmaxvalue _maxvalue) (`KismetMathLibrary.MaxOfIntArray` (`/Game/BP/BP_GameInstance.Speed_Array` (cast `/Game/BP/BP_GameInstance` (`GameplayStatics.GetGameInstance`) :!pure true))))
  (for (_ _array_index) _speed_array
    (`KismetArrayLibrary.Array_Insert` (`/Game/BP/BP_GameInstance.Speed_Array_0` (cast `/Game/BP/BP_GameInstance` (`GameplayStatics.GetGameInstance`) :!pure true)) _maxvalue _array_index)
    (`KismetArrayLibrary.Array_Set` _speed_array _indexofmaxvalue)))

(event `Roll_spd`
  (set `self.player_num` 0)
  (`self.Sort_Speed`)
  (for _index (range 4)
    (`KismetSystemLibrary.PrintString` (`KismetStringLibrary.Conv_IntToString` (`|GetArrayItem` (`/Game/BP/BP_GameInstance.Speed_Array_0` (cast `/Game/BP/BP_GameInstance` (`GameplayStatics.GetGameInstance`) :!pure true)) _index)))))

(event `atk_spd`
  (bind _player_num (`self.player_num`))
  (bind _speed_array_0 (`/Game/BP/BP_GameInstance.Speed_Array_0` (cast `/Game/BP/BP_GameInstance` (`GameplayStatics.GetGameInstance`) :!pure true)))
  ;[1 1 1] 通常攻撃によるスピードの変化
  (`KismetArrayLibrary.Array_Set` _speed_array_0 _player_num (`KismetMathLibrary.FTrunc` (* (`|GetArrayItem` _speed_array_0 _player_num) 1.0)))
  (`/Engine/EditorBlueprintResources/StandardMacros.IncrementInt` _player_num))

(event `Spc_spd`
  (bind _player_num (`self.player_num`))
  (bind _speed_array_0 (`/Game/BP/BP_GameInstance.Speed_Array_0` (cast `/Game/BP/BP_GameInstance` (`GameplayStatics.GetGameInstance`) :!pure true)))
  ;[1 1 1] とくぎによるスピードの変化
  (`KismetArrayLibrary.Array_Set` _speed_array_0 _player_num (`KismetMathLibrary.FTrunc` (* (`|GetArrayItem` _speed_array_0 _player_num) 0.5)))
  (`/Engine/EditorBlueprintResources/StandardMacros.IncrementInt` _player_num))

(fn `UserConstructionScript`)