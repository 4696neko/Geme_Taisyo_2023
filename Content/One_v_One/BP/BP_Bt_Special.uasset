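; BP_Bt_Special is a One_v_One battle helper that applies the effect of a player's item.
; PlayerItem checks quantity, then branches into heal, attack buff, defence buff or damage, without decrementing quantity.
; Results are written into the game instance's Hero or EnemyA struct, with a death flag check after damage.
; Heal and buff values derive from TargetEnemy's stats, and damage sets HP to item Atk minus enemy HP.
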(fn `Player_Item`
  (params (BP_Item :type "/Game/One_v_One/BP/BP_Item Structure (by ref)") (Target_Enemy :type "/Game/One_v_One/BP/BP_Character Structure (by ref)") (Target_Player :type "/Game/One_v_One/BP/BP_Character Structure (by ref)"))
  (bind (_quantity _itemname _atk _healhp _healmp _atkbuf _spd _defencebuf _atk_buf _defbuf _healbuf) (break `/Game/One_v_One/BP/BP_Item` BP_Item))
  (bind (_charactername _maxhp _nowhp _maxmp _nowmp _defultatk _nowatk _defultspd _nowspd _defultdef _nowdef) (break `/Game/One_v_One/BP/BP_Character` Target_Enemy))
  (bind _returnvalue (+ _healhp _nowhp))
  (bind _returnvalue_2 (+ _healmp _nowmp))
  (bind _asbp_one_v_one_instance (cast `/Game/One_v_One/BP/BP_One_V_OneInstance` (`GameplayStatics.GetGameInstance`) :!pure true))
  (if (> _quantity 0)
    (if _healbuf
      (if (or (>= _returnvalue _maxhp) (>= _returnvalue_2 _maxmp))
        (bind _structout (setmembers `/Game/One_v_One/BP/BP_Character` :`StructRef` Target_Player :`NowHP` _maxhp :`NowMP` _maxmp))
        (set `/Game/One_v_One/BP/BP_One_V_OneInstance.Hero` _structout _asbp_one_v_one_instance)
        (else
          (bind _structout_2 (setmembers `/Game/One_v_One/BP/BP_Character` :`StructRef` Target_Player :`NowHP` _returnvalue :`NowMP` _returnvalue_2))
          (set `/Game/One_v_One/BP/BP_One_V_OneInstance.Hero` _structout_2 _asbp_one_v_one_instance)))
      (elif _atk_buf
        (bind _structout_3 (setmembers `/Game/One_v_One/BP/BP_Character` :`StructRef` Target_Player :`NowAtk` (`KismetMathLibrary.FTrunc` (* _nowatk _atkbuf))))
        (set `/Game/One_v_One/BP/BP_One_V_OneInstance.Hero` _structout_3 _asbp_one_v_one_instance)
        (elif _defbuf
          (bind _structout_4 (setmembers `/Game/One_v_One/BP/BP_Character` :`StructRef` Target_Player :`NowDef` (`KismetMathLibrary.FTrunc` (* _nowdef _defencebuf))))
          (set `/Game/One_v_One/BP/BP_One_V_OneInstance.Hero` _structout_4 _asbp_one_v_one_instance)
          (else
            (bind _structout_5 (setmembers `/Game/One_v_One/BP/BP_Character` :`StructRef` Target_Enemy :`NowHP` (- _atk _nowhp)))
            (set `/Game/One_v_One/BP/BP_One_V_OneInstance.EnemyA` _structout_5 (cast `/Game/One_v_One/BP/BP_One_V_OneInstance` (`GameplayStatics.GetGameInstance`) :!pure true))
            (if (<= (`.NowHP_22_7C1D8F80417BE5B3F6BAC29D355D5182` (break `/Game/One_v_One/BP/BP_Character` Target_Enemy)) 0)
              (bind _structout_6 (setmembers `/Game/One_v_One/BP/BP_Character` :`StructRef` Target_Enemy :`Dead` true))
              (set `/Game/One_v_One/BP/BP_One_V_OneInstance.EnemyA` _structout_6 (cast `/Game/One_v_One/BP/BP_One_V_OneInstance` (`GameplayStatics.GetGameInstance`) :!pure true)))))))))

(fn `UserConstructionScript`)