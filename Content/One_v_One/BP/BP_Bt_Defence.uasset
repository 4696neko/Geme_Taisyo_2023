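; BP_Bt_Defence resolves an enemy's attack on the player in the One_v_One battle.
; Its PlayerDef event subtracts the player's NowDef from the enemy's truncated NowAtk times Rate, applying positive damage to NowHP or printing "MISS!!" otherwise.
; It then sets Dead when 0 <= NowHP, so the flag is raised for non-negative HP.
; Updated character structs are written to Hero on BP_One_V_OneInstance.
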(event `PlayerDef`
  (params (Enemy :type "/Game/One_v_One/BP/BP_Character Structure (by ref)") (TargetPlayer :type "/Game/One_v_One/BP/BP_Character Structure (by ref)"))
  (bind (_charactername _maxhp _nowhp _maxmp _nowmp _defultatk _nowatk _defultspd _nowspd _defultdef _nowdef _rate) (break `/Game/One_v_One/BP/BP_Character` Enemy))
  (bind (_charactername_2 _maxhp_2 _nowhp_2 _maxmp_2 _nowmp_2 _defultatk_2 _nowatk_2 _defultspd_2 _nowspd_2 _defultdef_2 _nowdef_2) (break `/Game/One_v_One/BP/BP_Character` TargetPlayer))
  (bind _returnvalue (- (`KismetMathLibrary.FTrunc` (* _nowatk _rate)) _nowdef_2))
  (if (> _returnvalue 0)
    (bind _structout (setmembers `/Game/One_v_One/BP/BP_Character` :`StructRef` TargetPlayer :`NowHP` (- _nowhp_2 _returnvalue)))
    (set `/Game/One_v_One/BP/BP_One_V_OneInstance.Hero` _structout (cast `/Game/One_v_One/BP/BP_One_V_OneInstance` (`GameplayStatics.GetGameInstance`) :!pure true))
    (else
      (`KismetSystemLibrary.PrintString` "MISS!!")))
  (if (<= 0 (`.NowHP_22_7C1D8F80417BE5B3F6BAC29D355D5182` (break `/Game/One_v_One/BP/BP_Character` TargetPlayer)))
    (bind _structout_2 (setmembers `/Game/One_v_One/BP/BP_Character` :`StructRef` TargetPlayer :`Dead` true))
    (set `/Game/One_v_One/BP/BP_One_V_OneInstance.Hero` _structout_2 (cast `/Game/One_v_One/BP/BP_One_V_OneInstance` (`GameplayStatics.GetGameInstance`) :!pure true))))

(fn `UserConstructionScript`)