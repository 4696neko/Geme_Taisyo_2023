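; BP_Battle is the turn controller for a one-versus-one battle, apparently unfinished.
; Attack has BP_Command pick a random enemy command, then compares both fighters' speeds in the game instance, with ties favoring the enemy.
; Enemy normal attacks run through BP_Bt_Atack after a text timeline, showing a result widget if the hero dies.
; Special and item branches are stubs, the hero branch handles only turn delay, and much older logic is disconnected.
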(event `Attack`
  (bind _textui (`self.TextUI`))
  (bind _asbp_one_v_one_instance (cast `/Game/One_v_One/BP/BP_One_V_OneInstance` (`GameplayStatics.GetGameInstance`) :!pure true))
  (bind _asbp_one_v_one_instance_2 (cast `/Game/One_v_One/BP/BP_One_V_OneInstance` (`GameplayStatics.GetGameInstance`) :!pure true))
  (bind _playerdelayturn (`/Game/One_v_One/BP/BP_One_V_OneInstance.PlayerDelayTurn` (cast `/Game/One_v_One/BP/BP_One_V_OneInstance` (`GameplayStatics.GetGameInstance`) :!pure true)))
  (bind _enemya (`/Game/One_v_One/BP/BP_One_V_OneInstance.EnemyA` _asbp_one_v_one_instance_2))
  (bind _hero (`/Game/One_v_One/BP/BP_One_V_OneInstance.Hero` _asbp_one_v_one_instance_2))
  ;[1 1 1] 攻撃時の処理
  (bind _outactors (`GameplayStatics.GetAllActorsOfClass` "/Game/One_v_One/BP/BP_Command.BP_Command_C"))
  (`/Game/One_v_One/BP/BP_Command.EnemyCommand` (cast `/Game/One_v_One/BP/BP_Command` (`|GetArrayItem` _outactors) :!pure true) (`KismetMathLibrary.RandomIntegerInRange` 0 2))
  (if (>= (`.NowSpd_30_EF77B80848F10B2EF7609FB691837994` (break `/Game/One_v_One/BP/BP_Character` _enemya)) (`.NowSpd_30_EF77B80848F10B2EF7609FB691837994` (break `/Game/One_v_One/BP/BP_Character` _hero)))
    (set `/Game/One_v_One/BP/BP_One_V_OneInstance.NowChara` _enemya _asbp_one_v_one_instance_2)
    (bind _returnvalue (`|CreateWidget` "/Game/One_v_One/UI/W_Text.W_Text_C"))
    (bind _output_get (set `self.TextUI` _returnvalue))
    (`UserWidget.AddToViewport` _output_get 0)
    (`Widget.SetVisibility` (`/Game/One_v_One/UI/W_Text.Player_enemyAttack` _output_get) "Hidden")
    (`Widget.SetVisibility` (`/Game/One_v_One/UI/W_Text.PlayerMP_None_Text` _output_get) "Hidden")
    (`Timeline|タイムライン_0` :!via `PlayFromStart`
      (:`Finished`
        (switch `int` (`.ComandNum_45_E2C8BE434526361EE38466BCF91BD0BC` (break `/Game/One_v_One/BP/BP_Character` (`/Game/One_v_One/BP/BP_One_V_OneInstance.EnemyA` (cast `/Game/One_v_One/BP/BP_One_V_OneInstance` (`GameplayStatics.GetGameInstance`) :!pure true))))
          (:`0`
            ;;[1 1 1] エネミー通常攻撃時の処理
            (bind _outactors_2 (`GameplayStatics.GetAllActorsOfClass` "/Game/One_v_One/BP/BP_Bt_Atack.BP_Bt_Atack_C"))
            (bind _asbp_bt_atack (cast `/Game/One_v_One/BP/BP_Bt_Atack` (`|GetArrayItem` _outactors_2)))
            (`/Game/One_v_One/BP/BP_Bt_Atack.EnemyAtk` _asbp_bt_atack (`/Game/One_v_One/BP/BP_One_V_OneInstance.EnemyA` _asbp_one_v_one_instance) (`/Game/One_v_One/BP/BP_One_V_OneInstance.Hero` _asbp_one_v_one_instance))
            (if (`.Dead_32_2DD09B514FB38163D3DCB285D46251D5` (break `/Game/One_v_One/BP/BP_Character` (`/Game/One_v_One/BP/BP_One_V_OneInstance.Hero` (cast `/Game/One_v_One/BP/BP_One_V_OneInstance` (`GameplayStatics.GetGameInstance`) :!pure true))))
              (`Widget.RemoveFromParent` _textui)
              (set `self.Command_Val` 0)
              (bind _returnvalue_2 (`|CreateWidget` "/Game/One_v_One/UI/W_TestResult.W_TestResult_C"))
              (bind _output_get_2 (set `self.ResultUI` _returnvalue_2))
              (`UserWidget.AddToViewport` _output_get_2 0)
              (`Widget.SetVisibility` (`/Game/One_v_One/UI/W_TestResult.WinText` _output_get_2) "Hidden")
              (else
                (`Widget.SetVisibility` (`/Game/One_v_One/UI/W_Text.Enemy_playerAttack` _textui) "Hidden"))))
          (:`1`
            ;;[1 1 1] エネミーとくぎ使用時の処理
            (bind _outactors_3 (`GameplayStatics.GetAllActorsOfClass` "/Game/One_v_One/BP/BP_Bt_Special.BP_Bt_Special_C")))
          (:`2`
            ;;[1 1 1] エネミーアイテム使用時の処理
            (bind _outactors_4 (`GameplayStatics.GetAllActorsOfClass` "/Game/One_v_One/BP/BP_Bt_Item.BP_Bt_Item_C"))))))
    (else
      (set `/Game/One_v_One/BP/BP_One_V_OneInstance.NowChara` _hero _asbp_one_v_one_instance_2)
      (if (`/Game/One_v_One/BP/BP_One_V_OneInstance.Player_DelayTurn` (cast `/Game/One_v_One/BP/BP_One_V_OneInstance` (`GameplayStatics.GetGameInstance`) :!pure true))
        (if (>= _playerdelayturn 1)
          (bind _returnvalue_3 (`|CreateWidget` "/Game/One_v_One/UI/W_TurnDelayText.W_TurnDelayText_C"))
          (bind _output_get_3 (set `self.DelayTurn` _returnvalue_3))
          (`UserWidget.AddToViewport` _output_get_3 0)
          (`Timeline|タイムライン_3` :!via `PlayFromStart`
            (:`Finished`
              (`/Engine/EditorBlueprintResources/StandardMacros.DecrementInt` _playerdelayturn))))
        (elif (== 0 4)
          (`|CreateWidget` null)
          (else
            (`|CreateWidget` null)))))))

(fn `UserConstructionScript`)