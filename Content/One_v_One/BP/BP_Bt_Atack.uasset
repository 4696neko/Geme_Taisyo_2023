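; BP_Bt_Atack is the battle attack calculator for one-on-one fights between the Hero and EnemyA.
; EnemyAtk and AtkPlayer mirror each other, subtracting the attacker's NowAtk times Rate, randomized by ±0.2 and truncated, from the target's NowHP.
; Each writes the target's BP_Character struct back to BP_One_V_OneInstance and sets its Dead flag when the HP check finds zero or below.
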(event `EnemyAtk`
  (params (Enemy :type "/Game/One_v_One/BP/BP_Character Structure (by ref)") (TargetPlayer :type "/Game/One_v_One/BP/BP_Character Structure (by ref)"))
  (bind (_charactername _maxhp _nowhp _maxmp _nowmp _defultatk _nowatk _defultspd _nowspd _defultdef _nowdef _rate) (break `/Game/One_v_One/BP/BP_Character` Enemy))
  ;[1 1 1] 攻撃時のダメージ計算
  ;;[1 1 1] 敵がプレイヤーに対して攻撃するとき
  (bind _structout (setmembers `/Game/One_v_One/BP/BP_Character` :`StructRef` TargetPlayer :`NowHP` (- (`.NowHP_22_7C1D8F80417BE5B3F6BAC29D355D5182` (break `/Game/One_v_One/BP/BP_Character` TargetPlayer)) (`KismetMathLibrary.FTrunc` (* _nowatk (+ _rate (`KismetMathLibrary.RandomFloatInRange` -0.2 0.2)))))))
  (set `/Game/One_v_One/BP/BP_One_V_OneInstance.Hero` _structout (cast `/Game/One_v_One/BP/BP_One_V_OneInstance` (`GameplayStatics.GetGameInstance`) :!pure true))
  (if (<= (`.NowHP_22_7C1D8F80417BE5B3F6BAC29D355D5182` (break `/Game/One_v_One/BP/BP_Character` TargetPlayer)) 0)
    (bind _structout_2 (setmembers `/Game/One_v_One/BP/BP_Character` :`StructRef` TargetPlayer :`Dead` true))
    (set `/Game/One_v_One/BP/BP_One_V_OneInstance.Hero` _structout_2 (cast `/Game/One_v_One/BP/BP_One_V_OneInstance` (`GameplayStatics.GetGameInstance`) :!pure true))))

(event `AtkPlayer`
  (params (Player :type "/Game/One_v_One/BP/BP_Character Structure (by ref)") (TargetEnemy :type "/Game/One_v_One/BP/BP_Character Structure (by ref)"))
  (bind (_charactername _maxhp _nowhp _maxmp _nowmp _defultatk _nowatk _defultspd _nowspd _defultdef _nowdef _rate) (break `/Game/One_v_One/BP/BP_Character` Player))
  ;[1 1 1] 攻撃時のダメージ計算
  ;;[1 1 1] プレイヤーが敵に対して攻撃するとき
  (bind _structout (setmembers `/Game/One_v_One/BP/BP_Character` :`StructRef` TargetEnemy :`NowHP` (- (`.NowHP_22_7C1D8F80417BE5B3F6BAC29D355D5182` (break `/Game/One_v_One/BP/BP_Character` TargetEnemy)) (`KismetMathLibrary.FTrunc` (* _nowatk (+ _rate (`KismetMathLibrary.RandomFloatInRange` -0.2 0.2)))))))
  (set `/Game/One_v_One/BP/BP_One_V_OneInstance.EnemyA` _structout (cast `/Game/One_v_One/BP/BP_One_V_OneInstance` (`GameplayStatics.GetGameInstance`) :!pure true))
  (if (<= (`.NowHP_22_7C1D8F80417BE5B3F6BAC29D355D5182` (break `/Game/One_v_One/BP/BP_Character` TargetEnemy)) 0)
    (bind _structout_2 (setmembers `/Game/One_v_One/BP/BP_Character` :`StructRef` TargetEnemy :`Dead` true))
    (set `/Game/One_v_One/BP/BP_One_V_OneInstance.EnemyA` _structout_2 (cast `/Game/One_v_One/BP/BP_One_V_OneInstance` (`GameplayStatics.GetGameInstance`) :!pure true))))

(fn `UserConstructionScript`)