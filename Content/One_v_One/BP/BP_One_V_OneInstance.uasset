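; BP_One_V_OneInstance holds the starting character, skill and item data for a one-on-one RPG-style battle.
; CreateCharacter builds Hero, EnemyA and EnemyB structs with maximum or default stats alongside current values.
; SetPlayer1Special and SetPlayer1Item fill Player 1's arrays of MP-costed special attacks and quantity-limited items, using hardcoded Japanese names.
; The functions only assign variables; this file contains no battle logic or calls to them.
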(fn `Create_Character`
  (set `self.Hero` (make `/Game/One_v_One/BP/BP_Character` "Hero" 100 100 50 50 10 10 10 10 10 10))
  (set `self.EnemyA` (make `/Game/One_v_One/BP/BP_Character` "EnemyA" 100 100 10 10 10 10 10 10 10 10))
  (set `self.EnemyB` (make `/Game/One_v_One/BP/BP_Character` "EnemyB" 200 200 30 30 20 20 5 5 15 15)))

(fn `SetPlayer1_Item`
  (set `self.Player1_Item` (`|MakeArray` (make `/Game/ProtoTest/BP/BP_Item` 3 "モロトフ" 30 0 0 1.0 20) (make `/Game/ProtoTest/BP/BP_Item` 5 "回復薬" 0 60 0 1.0 999 1.0 false false true) (make `/Game/ProtoTest/BP/BP_Item` 2 "魔力回復薬" 0 0 30 1.0 999 1.0 false false true) (make `/Game/ProtoTest/BP/BP_Item` 1 "力の丸薬" 0 0 0 2.0 999 1.0 true) (make `/Game/ProtoTest/BP/BP_Item` 1 "鎮痛剤" 0 0 0 1.0 0 1.5 false true))))

(fn `SetPlayer1_Special`
  (set `self.Player1_Sp` (`|MakeArray` (make `/Game/ProtoTest/BP/BP_SpecialAtk` "ふれいむ" 10 20 1.0 20) (make `/Game/ProtoTest/BP/BP_SpecialAtk` "ためる" 5 0 2.0 30 1.0 0 1.0 0 1.0 true false 1) (make `/Game/ProtoTest/BP/BP_SpecialAtk` "きりつける" 5 50) (make `/Game/ProtoTest/BP/BP_SpecialAtk` "いやす" 10 0 1.0 0 1.0 0 1.0 40 1.0 true) (make `/Game/ProtoTest/BP/BP_SpecialAtk` "きゅうしょづき" 15 50 1.0 20))))