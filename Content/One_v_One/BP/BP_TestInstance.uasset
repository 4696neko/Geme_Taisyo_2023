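; BP_TestInstance holds hard-coded test data for what appears to be a turn-based battle in One_v_One.
; CreateCharacter builds BPPlayer structs for Hero and two enemies flagged as Enemy, then stores them unsorted in SpdStruct.
; Each struct pairs base or max stats with current values for HP, MP, attack, speed and defense.
; SetPlayer1Special fills Player1Sp with Japanese-named special moves, each defined by name and MP cost.
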(fn `Create_Character`
  (set `self.Hero` (make `/Game/ProtoTest/BP/BP_Player` "Hero" 100 100 50 50 10 10 10 10 10 10))
  (set `self.EnemyA` (make `/Game/ProtoTest/BP/BP_Player` "EnemyA" 100 100 10 10 10 10 10 10 10 10 1.0 true))
  (set `self.EnemyB` (make `/Game/ProtoTest/BP/BP_Player` "EnemyB" 50 50 10 10 10 10 20 20 10 10 1.0 true))
  (set `self.Spd_Struct` (`|MakeArray` (`self.Hero`) (`self.EnemyA`) (`self.EnemyB`))))

(fn `SetPlayer1_Special`
  (set `self.Player1_Sp` (`|MakeArray` (make `/Game/ProtoTest/BP/BP_SpecialAtk` "ふれいむ" 10 20 1.0 20) (make `/Game/ProtoTest/BP/BP_SpecialAtk` "ためる" 5 0 2.0 30 1.0 0 1.0 0 1.0 true false 1) (make `/Game/ProtoTest/BP/BP_SpecialAtk` "きりつける" 5 50) (make `/Game/ProtoTest/BP/BP_SpecialAtk` "いやす" 10 0 1.0 0 1.0 0 1.0 40 1.0 true) (make `/Game/ProtoTest/BP/BP_SpecialAtk` "きゅうしょづき" 15 50 1.0 20))))