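; BP_Command picks the enemy's command in the One_v_One game from preset patterns.
; EnemyCommand switches on pattern number and EnemyTurn, passes a fixed command to SetEnemyCommand, then increments the turn.
; SetEnemyCommand writes that command into the EnemyA struct on BP_One_V_OneInstance.
; Only turns 0 and 1 have cases, so the above-2 check that resets EnemyTurn and EnemyCommandFlg is unreachable by counting up from zero.
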(event `EnemyCommand`
  (params (CommandNum :type Integer))
  (bind _enemyturn (`self.EnemyTurn`))
  (bind _enemyturn_2 (`self.EnemyTurn`))
  (bind _enemyturn_3 (`self.EnemyTurn`))
  (set `self.EnemyCommandFlg` true)
  (switch `int` CommandNum
    (:`0`
      (switch `int` (`self.EnemyTurn`)
        (:`0`
          (`self.Set_Enemy_Command` 0))
        (:`1`
          (`self.Set_Enemy_Command` 1)))
      (`/Engine/EditorBlueprintResources/StandardMacros.IncrementInt` _enemyturn_2
        (:`  `
          (if (> _enemyturn_2 2)
            (set `self.EnemyTurn` 0)
            (set `self.EnemyCommandFlg` false :!label _label)))))
    (:`1`
      (switch `int` (`self.EnemyTurn`)
        (:`0`
          (`self.Set_Enemy_Command` 0))
        (:`1`
          (`self.Set_Enemy_Command` 2)))
      (`/Engine/EditorBlueprintResources/StandardMacros.IncrementInt` _enemyturn_3
        (:`  `
          (if (> _enemyturn_3 2)
            (set `self.EnemyTurn` 0)
            (goto _label)))))
    (:`2`
      (switch `int` (`self.EnemyTurn`)
        (:`0`
          (`self.Set_Enemy_Command` 1))
        (:`1`
          (`self.Set_Enemy_Command` 1)))
      (`/Engine/EditorBlueprintResources/StandardMacros.IncrementInt` _enemyturn
        (:`  `
          (if (> _enemyturn 2)
            (set `self.EnemyTurn` 0)
            (goto _label)))))))

(fn `Set_Enemy_Command`
  (params (ComandNum :type Integer))
  (bind _asbp_one_v_one_instance (cast `/Game/One_v_One/BP/BP_One_V_OneInstance` (`GameplayStatics.GetGameInstance`) :!pure true))
  (bind _structout (setmembers `/Game/One_v_One/BP/BP_Character` :`StructRef` (`/Game/One_v_One/BP/BP_One_V_OneInstance.EnemyA` _asbp_one_v_one_instance) :`ComandNum` ComandNum))
  (set `/Game/One_v_One/BP/BP_One_V_OneInstance.EnemyA` _structout _asbp_one_v_one_instance))

(fn `UserConstructionScript`)