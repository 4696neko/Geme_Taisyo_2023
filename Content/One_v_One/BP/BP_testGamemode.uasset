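; Test game mode that drives a command menu with Attack, Special Attack, Item and Defense buttons.
; BeginPlay creates the menu widget, and Up/Down inputs move a wrapping index that UpDown, also run from Tick, shows as a red highlight.
; Function A, not called here, hides the menu, advances the command stage, opens Special or Item sub-widgets and sets a player selection.
; Sub-menu highlighting sits behind a top-level-only check, so it never runs.
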(event `self.ReceiveTick`
  (params (DeltaSeconds :type "Float (single-precision)"))
  (`UserWidget.AddToViewport` (stale `self.ReceiveBeginPlay` _output_get) 0 :!label _label)
  (`self.UpDown` :!label _label_2))

(event `self.ReceiveBeginPlay`
  (set `self.Command` 0)
  (set `self.Com_Button_UpDown` 0)
  (bind _returnvalue (`|CreateWidget` "/Game/ProtoTest/UI/Test＿UI.Test＿UI_C"))
  (bind _output_get (set `self.C_UI` _returnvalue))
  (goto _label))

(event `InputAction|Button_UP`
  (params (Key :type "Key Structure"))
  (bind _com_button_updown (`self.Com_Button_UpDown`))
  (:`Pressed`
    (if (== (`self.Command`) 0)
      (set `self.Com_Button_UpDown` (- _com_button_updown 1))
      (if (<= _com_button_updown 0)
        (set `self.Com_Button_UpDown` 4)
        (goto _label_2)))))

(event `InputAction|Button_DOWN`
  (params (Key :type "Key Structure"))
  (bind _com_button_updown (`self.Com_Button_UpDown`))
  (:`Pressed`
    (if (== (`self.Command`) 0)
      (set `self.Com_Button_UpDown` (+ _com_button_updown 1))
      (if (>= _com_button_updown 5)
        (set `self.Com_Button_UpDown` 1)
        (goto _label_2)))))

(fn `A`
  (bind _command (`self.Command`))
  (bind _command_2 (`self.Command`))
  (bind _returnvalue (+ _command_2 2))
  (if (<= _command 0)
    (set `self.Command` 0))
  (if (`KismetMathLibrary.InRange_FloatFloat` (`KismetMathLibrary.Conv_IntToDouble` _command) 0.0 2.0)
    (`Widget.SetVisibility` (`self.C_UI`) "Hidden")
    (switch `int` (`self.Com_Button_UpDown`)
      (:`1`
        (set `self.Select_Player` 0)
        (set `self.Command` _returnvalue)
        (if (== _command_2 2) :!label _label
          _))
      (:`2`
        (set `self.Command` (+ _command_2 1))
        (bind _returnvalue_2 (`|CreateWidget` "/Game/ProtoTest/UI/Test_Spe_UI.Test_Spe_UI_C"))
        (bind _output_get (set `self.SpeUI` _returnvalue_2))
        (`UserWidget.AddToViewport` _output_get 0)
        (switch `int` (`self.Sp_Button_UpDown`)
          (:`0`
            (set `self.Select_Player` 0))))
      (:`3`
        (set `self.Command` (+ _command_2 1))
        (bind _returnvalue_3 (`|CreateWidget` "/Game/ProtoTest/UI/Test_Item_UI.Test_Item_UI_C"))
        (bind _output_get_2 (set `self.Item_UI` _returnvalue_3))
        (`UserWidget.AddToViewport` _output_get_2 0)
        (switch `int` (`self.Item_Button_UpDown`)
          (:`0`
            (set `self.Select_Player` 0)
            (goto _label))
          (:`1`
            _)
          (:`2`
            _)
          (:`3`
            _)
          (:`4`
            _))
        (set `self.Select_Player` 1)
        (goto _label))
      (:`4`
        (set `self.Select_Player` 1)
        (set `self.Command` _returnvalue)
        (goto _label)))))

(fn `UpDown`
  (bind _c_ui (`self.C_UI`))
  (bind _speui (`self.SpeUI`))
  (bind _item_ui (`self.Item_UI`))
  (bind _com_button_updown (`self.Com_Button_UpDown`))
  (bind _command (`self.Command`))
  (bind _attackbutton (`/Game/ProtoTest/UI/Test＿UI.AttackButton` _c_ui))
  (if (== _command 0)
    (`Button.SetBackgroundColor` _attackbutton (struct :`R` 1.0 :`G` 1.0 :`B` 1.0 :`A` 1.0))
    (`Button.SetBackgroundColor` (`/Game/ProtoTest/UI/Test＿UI.SpacialAttackButton` _c_ui) (struct :`R` 1.0 :`G` 1.0 :`B` 1.0 :`A` 1.0))
    (`Button.SetBackgroundColor` (`/Game/ProtoTest/UI/Test＿UI.ItemButton` _c_ui) (struct :`R` 1.0 :`G` 1.0 :`B` 1.0 :`A` 1.0))
    (`Button.SetBackgroundColor` (`/Game/ProtoTest/UI/Test＿UI.DefenseButton` _c_ui) (struct :`R` 1.0 :`G` 1.0 :`B` 1.0 :`A` 1.0))
    (switch `int` (`self.Command`)
      (:`0`
        (switch `int` _com_button_updown
          (:`1`
            (`Button.SetBackgroundColor` _attackbutton (struct :`R` 1.0 :`A` 1.0)))
          (:`2`
            (`Button.SetBackgroundColor` (`/Game/ProtoTest/UI/Test＿UI.SpacialAttackButton` _c_ui) (struct :`R` 1.0 :`A` 1.0)))
          (:`3`
            (`Button.SetBackgroundColor` (`/Game/ProtoTest/UI/Test＿UI.ItemButton` _c_ui) (struct :`R` 1.0 :`A` 1.0)))
          (:`4`
            (`Button.SetBackgroundColor` (`/Game/ProtoTest/UI/Test＿UI.DefenseButton` _c_ui) (struct :`R` 1.0 :`A` 1.0)))))
      (:`1`
        (if (== _com_button_updown 1)
          (switch `int` (`self.Sp_Button_UpDown`)
            (:`1`
              (`Button.SetBackgroundColor` (`/Game/ProtoTest/UI/Test_Spe_UI.SpecialButton1` _speui) (struct :`R` 1.0 :`A` 1.0)))
            (:`2`
              (`Button.SetBackgroundColor` (`/Game/ProtoTest/UI/Test_Spe_UI.SpecialButton2` _speui) (struct :`R` 1.0 :`A` 1.0)))
            (:`3`
              (`Button.SetBackgroundColor` (`/Game/ProtoTest/UI/Test_Spe_UI.SpecialButton3` _speui) (struct :`R` 1.0 :`A` 1.0)))
            (:`4`
              (`Button.SetBackgroundColor` (`/Game/ProtoTest/UI/Test_Spe_UI.SpecialButton4` _speui) (struct :`R` 1.0 :`A` 1.0)))
            (:`5`
              (`Button.SetBackgroundColor` (`/Game/ProtoTest/UI/Test_Spe_UI.SpecialButton5` _speui) (struct :`R` 1.0 :`A` 1.0))))
          (else
            (switch `int` (`self.Item_Button_UpDown`)
              (:`1`
                (`Button.SetBackgroundColor` (`/Game/ProtoTest/UI/Test_Item_UI.ItemButton1` _item_ui) (struct :`R` 1.0 :`A` 1.0)))
              (:`2`
                (`Button.SetBackgroundColor` (`/Game/ProtoTest/UI/Test_Item_UI.ItemButton2` _item_ui) (struct :`R` 1.0 :`A` 1.0)))
              (:`3`
                (`Button.SetBackgroundColor` (`/Game/ProtoTest/UI/Test_Item_UI.ItemButton3` _item_ui) (struct :`R` 1.0 :`A` 1.0)))
              (:`4`
                (`Button.SetBackgroundColor` (`/Game/ProtoTest/UI/Test_Item_UI.ItemButton4` _item_ui) (struct :`R` 1.0 :`A` 1.0)))
              (:`5`
                (`Button.SetBackgroundColor` (`/Game/ProtoTest/UI/Test_Item_UI.ItemButton5` _item_ui) (struct :`R` 1.0 :`A` 1.0))))))))
    (elif (> _command 0)
      (set `self.Command` 0))))

(fn `UserConstructionScript`)